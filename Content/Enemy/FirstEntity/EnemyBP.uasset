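; Enemy AI character that roams, chases the player on sight and performs a jumpscare on catching them.
; Pawn sensing triggers AIMoveTo, chase audio and higher speed, while Tick handles losing sight and random reachable-point wandering after delays.
; A successful move starts a self-calling delayed loop that turns the player and camera toward the enemy, plays a montage, fades out and calls OpenLevelAfterJumpscare with the current level.
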(event OnSeePawn(PawnSensing)
  (params (Pawn :type Pawn%20Object%20Reference))
  ;[1 1 1] Ai Chase
  (bind _asbp_first_person_character (Utilities|Casting|CastToBP_FirstPersonCharacter Pawn))
  (if (not (Variables|Default|GetCaught?))
    (Utilities|FlowControl|Sequence
      (:then_0
        (Variables|Default|SetCan%20See%20Enemy? true)
        (Variables|Default|SetIsChasing? true)
        (AI|AIMoveTo self "0, 0, 0" _asbp_first_person_character 5.0 false
          (:then
            (Utilities|FlowControl|DoOnce false
              (:Completed
                (Audio|Components|Audio|Play (Variables|Default|GetAudio) 0.25)
                (Components|Timeline|SetPlayRate (Variables|Character|GetMesh) 12.5)
                (Variables|/Script/Engine.CharacterMovementComponent|SetMaxWalkSpeed (Variables|Character|GetCharacterMovement) 8e+02))))
          (:OnSuccess
            (CallFunction|CatchPlayer))))
      (:then_1
        (Utilities|FlowControl|RetriggerableDelay 0.6)
        (Variables|Default|SetCan%20See%20Enemy? false)))))

(event Custom|CatchPlayer
  (bind _returnvalue (Game|GetPlayerController 0))
  (Variables|Default|SetCaught? true)
  (Variables|Default|SetShouldLoop? true)
  (bind _asbp_first_person_character (Utilities|Casting|CastToBP_FirstPersonCharacter (Game|GetPlayerCharacter 0)))
  (if (Variables|Default|GetShouldLoop?)
    (Utilities|FlowControl|Delay 0.001)
    (Transformation|SetActorRotation _asbp_first_person_character (Math|Interpolation|RInterpTo (Transformation|GetActorRotation _asbp_first_person_character) (Math|Rotator|FindLookatRotation (Transformation|GetActorLocation _asbp_first_person_character) (Transformation|GetActorLocation)) (Utilities|Time|GetWorldDeltaSeconds) 5.0))
    (Pawn|SetControlRotation _returnvalue (Math|Interpolation|RInterpTo (Pawn|GetControlRotation _returnvalue :!class /Script/Engine.Controller) (Math|Rotator|FindLookatRotation (Transformation|GetActorLocation _asbp_first_person_character) (Transformation|GetActorLocation)) (Utilities|Time|GetWorldDeltaSeconds) 5.0))
    (CallFunction|RotationLoop)
    (Utilities|FlowControl|DoOnce false :!label _label
      (:Completed
        (Utilities|FlowControl|Sequence
          (:then_0
            (Animation|PlayAnimMontage 0 0.7 "None")
            (Components|Timeline|SetPlayRate (Variables|Character|GetMesh) 25.0)
            (Utilities|FlowControl|Delay 0.2)
            (CameraFades|StartCameraFade :self (Game|GetPlayerCameraManager 0) :ToAlpha 1.0 :Duration 0.5 :bShouldFadeAudio true :bHoldWhenFinished true)
            (bind _returnvalue_2 (Game|GetCurrentLevelName true))
            (Class|BackroomsDeath|OpenLevelAfterJumpscare (Utilities|String|StringToName _returnvalue_2))
            (Variables|Default|SetCaught? false))
          (:then_1
            (Utilities|FlowControl|Delay 0.35)
            (Variables|Default|SetShouldLoop? false)
            (goto _label Reset)))))))

(event Custom|RotationLoop
  (bind _returnvalue (Game|GetPlayerController 0))
  (if (Variables|Default|GetShouldLoop?)
    (Utilities|FlowControl|Delay 0.001)
    (Transformation|SetActorRotation (stale Custom|CatchPlayer _asbp_first_person_character) (Math|Interpolation|RInterpTo (Transformation|GetActorRotation (stale Custom|CatchPlayer _asbp_first_person_character)) (Math|Rotator|FindLookatRotation (Transformation|GetActorLocation (stale Custom|CatchPlayer _asbp_first_person_character)) (Transformation|GetActorLocation)) (Utilities|Time|GetWorldDeltaSeconds) 5.0))
    (Pawn|SetControlRotation _returnvalue (Math|Interpolation|RInterpTo (Pawn|GetControlRotation _returnvalue :!class /Script/Engine.Controller) (Math|Rotator|FindLookatRotation (Transformation|GetActorLocation (stale Custom|CatchPlayer _asbp_first_person_character)) (Transformation|GetActorLocation)) (Utilities|Time|GetWorldDeltaSeconds) 5.0))
    (CallFunction|RotationLoop)
    (Utilities|FlowControl|DoOnce false :!label _label
      (:Completed
        (Utilities|FlowControl|Sequence
          (:then_0
            (Animation|PlayAnimMontage 0 0.7 "None")
            (Components|Timeline|SetPlayRate (Variables|Character|GetMesh) 25.0)
            (Utilities|FlowControl|Delay 0.2)
            (CameraFades|StartCameraFade :self (Game|GetPlayerCameraManager 0) :ToAlpha 1.0 :Duration 0.5 :bShouldFadeAudio true :bHoldWhenFinished true)
            (bind _returnvalue_2 (Game|GetCurrentLevelName true))
            (Class|BackroomsDeath|OpenLevelAfterJumpscare (Utilities|String|StringToName _returnvalue_2))
            (Variables|Default|SetCaught? false))
          (:then_1
            (Utilities|FlowControl|Delay 0.35)
            (Variables|Default|SetShouldLoop? false)
            (goto _label Reset)))))))

(event EventBeginPlay
  ;[1 1 1] Create Audio Reference
  (bind _returnvalue (AddComponent|AddAudioComponent false))
  (Audio|Components|Audio|Stop _returnvalue)
  (Variables|Default|SetAudio _returnvalue))

(event EventTick
  (params (DeltaSeconds :type Float%20%28single-precision%29))
  ;[1 1 1] Ai Chase
  (if (not (Variables|Default|GetCaught?))
    (Utilities|FlowControl|Sequence
      (:then_0
        (if (not (Variables|Default|GetCan%20See%20Enemy?))
          (Utilities|FlowControl|Delay 0.4)
          (if (not (Variables|Default|GetCan%20See%20Enemy?))
            (Audio|Components|Audio|FadeOut (Variables|Default|GetAudio) 5.0 0.0 "Linear" :!class /Script/Engine.AudioComponent)
            (Variables|Default|SetIsChasing? false)
            (Utilities|FlowControl|DoOnce false) ; enters at Reset
          )))
      (:then_1
        (if (not (Variables|Default|GetIsChasing?))
          (Utilities|FlowControl|Delay (Math|Random|RandomFloatinRange 2.0 8.0))
          (AI|AIMoveTo self (.RandomLocation (AI|Navigation|GetRandomReachablePointinRadius (Transformation|GetActorLocation) 2.5e+04 0 0)) 0 5.0 false))))))

(fn ConstructionScript)