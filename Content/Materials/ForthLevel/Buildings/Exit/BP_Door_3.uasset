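; BP_Door_3 is a locked exit door that the first-person player breaks through with a key.
; A box overlap stores the character, enables E input and opens a gate, and leaving reverses the input and gate.
; Pressing E with HasKey set destroys the door, plays a break sound and spawns BP_Door_7_Collce at its transform.
; Without the key, E plays a locked sound.
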(event OnComponentBeginOverlap(Box)
  (params (OverlappedComponent :type Primitive%20Component%20Object%20Reference) (OtherActor :type Actor%20Object%20Reference) (OtherComp :type Primitive%20Component%20Object%20Reference) (OtherBodyIndex :type Integer) (bFromSweep :type Boolean) (SweepResult :type Hit%20Result%20Structure%20%28by%20ref%29))
  (bind _asbp_first_person_character (Utilities|Casting|CastToBP_FirstPersonCharacter OtherActor))
  (Input|EnableInput (Game|GetPlayerController 0))
  (Utilities|FlowControl|Gate true) ; enters at Open
)

(event OnComponentEndOverlap(Box)
  (params (OverlappedComponent :type Primitive%20Component%20Object%20Reference) (OtherActor :type Actor%20Object%20Reference) (OtherComp :type Primitive%20Component%20Object%20Reference) (OtherBodyIndex :type Integer))
  (Utilities|Casting|CastToBP_FirstPersonCharacter OtherActor)
  (Input|DisableInput (Game|GetPlayerController 0))
  (Utilities|FlowControl|Gate true) ; enters at Close
)

(event EventBeginPlay)

(event Input|KeyboardEvents|E
  (params (Key :type Key%20Structure))
  (:Pressed
    (if (Variables|/Game/FirstPerson/Blueprints/BP_FirstPersonCharacter.BP_FirstPersonCharacter_C|GetHasKey? (stale OnComponentBeginOverlap(Box) _asbp_first_person_character))
      (Utilities|FlowControl|Gate true
        (:Exit
          (Actor|DestroyActor)
          (Audio|PlaySoundatLocation "/Game/Sounds/FX/break.break" (Transformation|GetActorLocation) "0, 0, 0" 1.0 1.0 0.0 0 0 0 0)
          (Game|SpawnActorfromClass "/Game/Materials/ForthLevel/Buildings/Exit/BP_Door_7_Collce.BP_Door_7_Collce_C" (Transformation|GetActorTransform) "AlwaysSpawn" 0 0)))
      (else
        (Audio|PlaySoundatLocation "/Game/Sounds/FX/locked.locked" (Transformation|GetActorLocation) "0, 0, 0" 1.0 1.0 0.0 0 0 0 0)))))

(fn ConstructionScript)