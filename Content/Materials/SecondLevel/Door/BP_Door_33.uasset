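; Key-locked double door that the player toggles with E while standing in its Box trigger, which enables and disables input.
; E checks the character's HasKey, which BeginPlay resets to false, and plays a locked sound without it.
; With the key, the DoorRotation timeline swings both leaves in opposite directions or reverses, based on DoorClosed updated in Tick.
; A DoOnce limits the unlock sound to the first opening.
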(event OnComponentBeginOverlap(Box)
  (params (OverlappedComponent :type Primitive%20Component%20Object%20Reference) (OtherActor :type Actor%20Object%20Reference) (OtherComp :type Primitive%20Component%20Object%20Reference) (OtherBodyIndex :type Integer) (bFromSweep :type Boolean) (SweepResult :type Hit%20Result%20Structure%20%28by%20ref%29))
  (bind _asbp_first_person_character (Utilities|Casting|CastToBP_FirstPersonCharacter OtherActor))
  (Input|EnableInput (Game|GetPlayerController 0)))

(event OnComponentEndOverlap(Box)
  (params (OverlappedComponent :type Primitive%20Component%20Object%20Reference) (OtherActor :type Actor%20Object%20Reference) (OtherComp :type Primitive%20Component%20Object%20Reference) (OtherBodyIndex :type Integer))
  (Utilities|Casting|CastToBP_FirstPersonCharacter OtherActor)
  (Input|DisableInput (Game|GetPlayerController 0)))

(event EventBeginPlay
  (Utilities|FlowControl|DoOnce false
    (:Completed
      (bind _asbp_first_person_character (Utilities|Casting|CastToBP_FirstPersonCharacter (Game|GetPlayerCharacter 0)))
      (Variables|/Game/FirstPerson/Blueprints/BP_FirstPersonCharacter.BP_FirstPersonCharacter_C|SetHasKey? _asbp_first_person_character false))))

(event Collision|EventActorBeginOverlap
  (params (OtherActor :type Actor%20Object%20Reference)))

(event EventTick
  (params (DeltaSeconds :type Float%20%28single-precision%29))
  (Variables|Default|SetDoorClosed (< (stale Input|KeyboardEvents|E _door) 1.0)))

(event Input|KeyboardEvents|E
  (params (Key :type Key%20Structure :default "None"))
  (:Pressed
    (if (Variables|/Game/FirstPerson/Blueprints/BP_FirstPersonCharacter.BP_FirstPersonCharacter_C|GetHasKey? (stale OnComponentBeginOverlap(Box) _asbp_first_person_character))
      (if (Variables|Default|GetDoorClosed)
        (bind _door (Timeline|Door%20Rotation Play)
          (:Update
            (Transformation|SetRelativeLocationAndRotation (Variables|Default|GetDoorL) "0,507.000000, 0" (Math|Rotator|MakeRotator 0.0 0.0 _door) false false)
            (Transformation|SetRelativeLocationAndRotation (Variables|Default|GetDoorR) "0,-489.000000, 0" (* (Math|Rotator|MakeRotator 0.0 0.0 _door) -1.0) false false)
            (Utilities|FlowControl|DoOnce false
              (:Completed
                (Audio|PlaySoundatLocation "/Game/Sounds/FX/unlock.unlock" (Transformation|GetWorldLocation (Variables|Default|GetBox)) "0, 0, 0" 1.0 1.0 0.0 0 0 0 0)))))
        (else
          (Timeline|Door%20Rotation Reverse)))
      (else
        (Audio|PlaySoundatLocation "/Game/Sounds/FX/locked.locked" (Transformation|GetActorLocation) "0, 0, 0" 1.0 1.0 0.0 0 0 0 0)))))

(fn ConstructionScript)