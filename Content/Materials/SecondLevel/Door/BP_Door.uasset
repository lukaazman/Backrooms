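; BP_Door is a double door that opens and closes when the player presses E.
; A DoorRotation timeline swings DoorL and DoorR to opposite yaws at fixed offsets, playing or reversing based on DoorClosed.
; Tick sets DoorClosed whenever the timeline value is below 1.
; The Box trigger enables player 0 input on begin overlap and also on end overlap, so input is never disabled after leaving.
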(event OnComponentBeginOverlap(Box)
  (params (OverlappedComponent :type Primitive%20Component%20Object%20Reference) (OtherActor :type Actor%20Object%20Reference) (OtherComp :type Primitive%20Component%20Object%20Reference) (OtherBodyIndex :type Integer) (bFromSweep :type Boolean) (SweepResult :type Hit%20Result%20Structure%20%28by%20ref%29))
  (Input|EnableInput (Game|GetPlayerController 0)))

(event OnComponentEndOverlap(Box)
  (params (OverlappedComponent :type Primitive%20Component%20Object%20Reference) (OtherActor :type Actor%20Object%20Reference) (OtherComp :type Primitive%20Component%20Object%20Reference) (OtherBodyIndex :type Integer))
  (Input|EnableInput (Game|GetPlayerController 0)))

(event EventBeginPlay)

(event Collision|EventActorBeginOverlap
  (params (OtherActor :type Actor%20Object%20Reference)))

(event EventTick
  (params (DeltaSeconds :type Float%20%28single-precision%29))
  (Variables|Default|SetDoorClosed (< (stale Input|KeyboardEvents|E _door) 1.0)))

(event Input|KeyboardEvents|E
  (params (Key :type Key%20Structure :default "None"))
  (:Pressed
    (if (Variables|Default|GetDoorClosed)
      (bind _door (Timeline|Door%20Rotation Play)
        (:Update
          (Transformation|SetRelativeLocationAndRotation (Variables|Default|GetDoorL) "0,507.000000, 0" (Math|Rotator|MakeRotator 0.0 0.0 _door) false false)
          (Transformation|SetRelativeLocationAndRotation (Variables|Default|GetDoorR) "0,-489.000000, 0" (* (Math|Rotator|MakeRotator 0.0 0.0 _door) -1.0) false false)))
      (else
        (Timeline|Door%20Rotation Reverse)))))

(fn ConstructionScript)